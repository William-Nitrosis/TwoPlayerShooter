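; BP_Kar98k is a Kar98k rifle weapon that sets magazine size, ammo and fire rate on BeginPlay and counts down a shot cooldown on Tick.
; AttackStart only prints a debug string, and FireStart is empty.
; Disconnected firing logic would check ammo and cooldown, spawn a bullet at the muzzle along the parent player's camera rotation, and toggle Firing in ABP_Kar98k.
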(event `self.ReceiveBeginPlay`
  (bind _output_get (set `self.MagSize` 5))
  (set `self.CurrentAmmo` _output_get)
  (set `self.RateOfFire` 1.2))

(event `self.ReceiveTick`
  (params (DeltaSeconds :type "Float (single-precision)"))
  (set `self.ShotCooldown` (- (`self.ShotCooldown`) (`GameplayStatics.GetWorldDeltaSeconds`))))

(event `WeaponInterface.AttackStart`
  (`KismetSystemLibrary.PrintString` "Hello"))

(fn `FireStart`)

(fn `UserConstructionScript`
  (`parent.UserConstructionScript`))