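; Kar98k rifle weapon Blueprint that handles firing, reloading and ironsight scoping for the player.
; Firing and reload set flags on the rifle's AnimBP and clear ReadyToFire, which is not restored in this graph.
; Each shot spawns a projectile at the muzzle along the ironsight camera's rotation and applies randomized, timeline-driven controller recoil.
; Scoping blends the view target between rifle and character, toggling controller pitch rotation.
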(event `self.ReceiveTick`
  (params (DeltaSeconds :type "Float (single-precision)"))
  (`KismetSystemLibrary.PrintString` (`KismetStringLibrary.Conv_BoolToString` (`self.ReadyToFire`)) true true (struct :`G` 0.66 :`B` 1.0 :`A` 1.0) 0.001))

(event `WeaponInterface.Reload`
  (bind _asabp_kar_98k_new (cast `/Game/Developer/Weapons/Kar98K/New/ABP_Kar98k_new` (`SkeletalMeshComponent.GetAnimInstance` (`self.SkeletalMesh`))))
  (if (and (not (`/Game/Developer/Weapons/Kar98K/New/ABP_Kar98k_new.Firing` _asabp_kar_98k_new)) (!= (`self.CurrentAmmo`) (`self.MagSize`)) (`self.ReadyToFire`))
    (bind _asabp_kar_98k_new_2 (cast `/Game/Developer/Weapons/Kar98K/New/ABP_Kar98k_new` (`SkeletalMeshComponent.GetAnimInstance` (`self.SkeletalMesh`))))
    (set `/Game/Developer/Weapons/Kar98K/New/ABP_Kar98k_new.CallReload` true _asabp_kar_98k_new_2)
    (set `self.ReadyToFire` false)))

(event `WeaponInterface.AttackEnd`
  (bind _asabp_kar_98k_new (cast `/Game/Developer/Weapons/Kar98K/New/ABP_Kar98k_new` (`SkeletalMeshComponent.GetAnimInstance` (`self.SkeletalMesh`))))
  (set `/Game/Developer/Weapons/Kar98K/New/ABP_Kar98k_new.Firing` false _asabp_kar_98k_new))

(event `WeaponInterface.AttackStart`
  (bind _recoil (`self.Recoil`))
  (bind _returnvalue (/ _recoil 3.0))
  (if (`self.ReadyToFire`)
    (`KismetSystemLibrary.PrintString` "Firing")
    (set `self.ReadyToFire` false)
    (bind _asabp_kar_98k_new (cast `/Game/Developer/Weapons/Kar98K/New/ABP_Kar98k_new` (`SkeletalMeshComponent.GetAnimInstance` (`self.SkeletalMesh`))))
    (set `/Game/Developer/Weapons/Kar98K/New/ABP_Kar98k_new.Firing` true _asabp_kar_98k_new)
    (`GameplayStatics.PlaySoundAtLocation` "/Game/WW2_Kar98k/Audio/SD_Kar98k_Fire_Cue.SD_Kar98k_Fire_Cue" (`SceneComponent.K2_GetComponentLocation` (`self.Muzzle`)))
    (`/Engine/EditorBlueprintResources/StandardMacros.DecrementInt` (`self.CurrentAmmo`)
      (:`  `
        (`self.Spawn bullet`)
        ;[1 1 1] Recoil
        (bind _asmy_player_character_2 (cast `/Game/MyPlayerCharacter2` (`GameplayStatics.GetPlayerCharacter` 0)))
        (bind (_direction _float_tick) (`Timeline|Recoil timeline` :!via `PlayFromStart`)
          (:`Update`
            (`Pawn.AddControllerYawInput` _asmy_player_character_2 (`KismetMathLibrary.Lerp` 0.0 (`KismetMathLibrary.RandomFloatInRange` (* _returnvalue -1.0) _returnvalue) _float_tick))
            (`Pawn.AddControllerPitchInput` _asmy_player_character_2 (`KismetMathLibrary.Lerp` 0.0 (`KismetMathLibrary.RandomFloatInRange` (* _recoil -1.0) (* _recoil -0.3)) _float_tick))))))))

(event `WeaponInterface.ScopeIn`
  ;[1 1 1] Scoping in and out
  (bind _asmy_player_character_2 (cast `/Game/MyPlayerCharacter2` (`GameplayStatics.GetPlayerCharacter` 0)))
  (`PlayerController.SetViewTargetWithBlend` (`GameplayStatics.GetPlayerController` 0) self 0.2 "VTBlend_Linear" 0.0 false)
  (set `Pawn.bUseControllerRotationPitch` true _asmy_player_character_2))

(event `WeaponInterface.ScopeOut`
  ;[1 1 1] Scoping in and out
  (bind _asmy_player_character_2 (cast `/Game/MyPlayerCharacter2` (`GameplayStatics.GetPlayerCharacter` 0)))
  (`PlayerController.SetViewTargetWithBlend` (`GameplayStatics.GetPlayerController` 0) _asmy_player_character_2 0.2 "VTBlend_Linear" 0.0 false)
  (set `Pawn.bUseControllerRotationPitch` false _asmy_player_character_2))

(fn `Spawn bullet`
  (`|SpawnActorFromClass` "/Game/Developer/Weapons/Bullet/BP_bullet_projectile.BP_bullet_projectile_C" (`KismetMathLibrary.MakeTransform` (`SceneComponent.K2_GetComponentLocation` (`self.Muzzle`)) (`SceneComponent.K2_GetComponentRotation` (`self.Camera_ironsight`))) "AlwaysSpawn" "OverrideRootScale" null null))

(fn `UserConstructionScript`
  (`parent.UserConstructionScript`))